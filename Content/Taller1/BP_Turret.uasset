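; BP_Turret is a turret actor that turns toward a target and fires bullets at a regular interval.
; Each tick it eases its rotation toward ViewActor using a look-at rotation with pitch zeroed and a small fixed lerp alpha, so turn speed depends on frame rate.
; A looping timer set on BeginPlay, paced by TimeToShoot, spawns a Bullet at the Cube component's location and rotation with a fixed speed.
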(event `ShootEvent_Event`
  (`|SpawnActorFromClass` (`self.bullet`) (`KismetMathLibrary.MakeTransform` (.location (`SceneComponent.K2_GetComponentToWorld` (`self.Cube`))) (.rotation (`SceneComponent.K2_GetComponentToWorld` (`self.Cube`)))) "Undefined" "OverrideRootScale" null 750.0 null))

(event `self.ReceiveBeginPlay`
  (`KismetSystemLibrary.K2_SetTimerDelegate` (delegate `ShootEvent_Event`) (`self.timeToShoot`) true))

(event `self.ReceiveTick`
  (params (DeltaSeconds :type "Float (single-precision)"))
  (`self.K2_SetActorRotation` (`KismetMathLibrary.RLerp` (`self.K2_GetActorRotation`) (`KismetMathLibrary.MakeRotator` (.roll (`KismetMathLibrary.FindLookAtRotation` (`self.K2_GetActorLocation`) (`self.K2_GetActorLocation` (`self.viewActor`)))) 0.0 (.yaw (`KismetMathLibrary.FindLookAtRotation` (`self.K2_GetActorLocation`) (`self.K2_GetActorLocation` (`self.viewActor`))))) 0.01 true)))

(fn `UserConstructionScript`)
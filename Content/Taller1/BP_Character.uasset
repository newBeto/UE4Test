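; BP_Character is a character Blueprint that moves along the world X and Y axes from player axis input.
; Each Tick reads the MoveForward and MoveRight axis values, scales them by Speed and delta time, and offsets the actor location.
; Movement sets the location directly without sweep, so this move does not stop at blocking collision.
; The axis events are empty, and two per-axis swept moves remain disconnected.
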(event `self.ReceiveTick`
  (params (DeltaSeconds :type "Float (single-precision)"))
  (`self.K2_SetActorLocation` (+ (`KismetMathLibrary.MakeVector` (* (`self.GetInputAxisValue`) (`self.speed`) DeltaSeconds) (* (`self.GetInputAxisValue`) (`self.speed`) DeltaSeconds)) (`self.K2_GetActorLocation`))))

(event `InputAxis|MoveForward`
  (params (AxisValue :type "Float (single-precision)")))

(event `InputAxis|MoveRight`
  (params (AxisValue :type "Float (single-precision)")))

(fn `UserConstructionScript`)
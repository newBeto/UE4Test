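; BP_Bullet is a projectile Actor that flies along its forward vector and destroys itself on overlap or when a short timer expires.
; Tick moves it by Speed scaled by delta time, without sweeping.
; A StaticMesh overlap prints debug text, applies a swept offset to the other Actor, then destroys the bullet.
; That offset is currently zero because the horizontal knockback direction calculation is left unconnected.
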(event `TimerToDestroy_Event`
  (`self.K2_DestroyActor`))

(event `self.ReceiveBeginPlay`
  (`KismetSystemLibrary.K2_SetTimerDelegate` (delegate `TimerToDestroy_Event`) 2.0))

(event `self.ReceiveTick`
  (params (DeltaSeconds :type "Float (single-precision)"))
  (`self.K2_SetActorLocation` (+ (* (`KismetMathLibrary.GetForwardVector` (`self.K2_GetActorRotation`)) (* DeltaSeconds (`self.speed`))) (`self.K2_GetActorLocation`))))

(event `self.StaticMesh.OnComponentBeginOverlap`
  (params (OverlappedComponent :type "PrimitiveComponent Object Reference") (OtherActor :type "Actor Object Reference") (OtherComp :type "PrimitiveComponent Object Reference") (OtherBodyIndex :type Integer) (bFromSweep :type Boolean) (SweepResult :type "HitResult Structure (by ref)"))
  (`KismetSystemLibrary.PrintString` "test")
  (`KismetSystemLibrary.PrintString` "test")
  (`self.K2_SetActorLocation` OtherActor (+ (`self.K2_GetActorLocation` OtherActor) (* (0.0 0.0 0.0) 10.0)) true false)
  (`self.K2_DestroyActor`))

(fn `UserConstructionScript`)